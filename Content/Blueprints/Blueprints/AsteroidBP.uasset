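; AsteroidBP is an asteroid actor that glides at constant speed toward a stored target point.
; Tick normalizes the direction from its location to that vector variable and applies a delta-time-scaled step through SetActorLocationAndRotation.
; The code that would fetch the target from AsteroidSpawningPoint_BP is disconnected and never runs, so this graph never sets the variable.
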(event EventBeginPlay)

(event Collision|EventActorBeginOverlap
  (params (OtherActor :type Actor%20Object%20Reference)))

(event EventTick
  (params (DeltaSeconds :type Float%20%28single-precision%29))
  (bind _returnvalue (Transformation|GetActorLocation))
  (Transformation|SetActorLocationAndRotation (+ (* (* (Math|Vector|Normalize (- (stale _location) _returnvalue)) DeltaSeconds) 1e+02) _returnvalue) "0, 0, 0"))

(fn ConstructionScript)