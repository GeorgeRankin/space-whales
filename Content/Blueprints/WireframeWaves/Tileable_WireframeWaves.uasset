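; Endless-runner floor tile for the space whales game, scattered with asteroids and space whales.
; The construction script adds both as child actor components at random points inside SpawnBox.
; When SpaceshipBP overlaps EndTrigger, the tile asks SpaceWhalesGameMode to add another floor tile, then destroys itself after a short delay.
; GetAttachTransform exposes the AttachPoint world transform, presumably for chaining the next tile.
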(event OnComponentBeginOverlap(EndTrigger)
  (params (OverlappedComponent :type Primitive%20Component%20Object%20Reference) (OtherActor :type Actor%20Object%20Reference) (OtherComp :type Primitive%20Component%20Object%20Reference) (OtherBodyIndex :type Integer) (bFromSweep :type Boolean) (SweepResult :type Hit%20Result%20Structure%20%28by%20ref%29))
  ;[1 1 1] Tiling the Platforms
  (Utilities|Casting|CastToSpaceshipBP OtherActor)
  (bind _asspace_whales_game_mode (Utilities|Casting|CastToSpaceWhalesGameMode (Game|GetGameMode)))
  (Default|AddFloorTile _asspace_whales_game_mode)
  (Utilities|FlowControl|Delay 5.0)
  (Actor|DestroyActor))

(event EventBeginPlay)

(event Collision|EventActorBeginOverlap
  (params (OtherActor :type Actor%20Object%20Reference)))

(event EventTick
  (params (DeltaSeconds :type Float%20%28single-precision%29)))

(fn ConstructionScript
  (CallFunction|SpawnAsteroidsin3D)
  (CallFunction|SpawnSpaceWhalesin3D))

(fn GetAttachTransform
  (return (Transformation|GetWorldTransform (Variables|Default|GetAttachPoint))))

(fn SpawnAsteroidsin3D
  (bind _spawnbox (Variables|Default|GetSpawnBox))
  (for _index (range 0 4)
    (AddComponent|AddChildActorComponent false (Math|Conversions|ToTransform(Vector) (Math|Random|RandomPointinBoundingBox (Variables|/Script/Engine.SceneComponent|GetRelativeLocation _spawnbox) (Variables|/Script/Engine.BoxComponent|GetBoxExtent _spawnbox))))))

(fn SpawnSpaceWhalesin3D
  (bind _spawnbox (Variables|Default|GetSpawnBox))
  (for _index (range 0 2)
    (AddComponent|AddChildActorComponent false (Math|Conversions|ToTransform(Vector) (Math|Random|RandomPointinBoundingBox (Variables|/Script/Engine.SceneComponent|GetRelativeLocation _spawnbox) (Variables|/Script/Engine.BoxComponent|GetBoxExtent _spawnbox))))))